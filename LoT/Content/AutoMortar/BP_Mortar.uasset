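; BP_Mortar is an auto mortar actor built from a body, a turret dome and a barrel mesh.
; The construction script assigns the static meshes to the three mesh components.
; On BeginPlay it initialises its TankAiming component with the barrel and turret, handing the aiming to that component.
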(event EventBeginPlay
  (Class|TankAimingComponent|Initialise (Variables|Default|GetTankAiming) (Variables|Default|GetMBarrel) (Variables|Default|GetMTurret)))

(fn ConstructionScript
  (Components|StaticMesh|SetStaticMesh (Variables|Default|GetMortar) "/Game/AutoMortar/mortar_body.mortar_body")
  (Components|StaticMesh|SetStaticMesh (Variables|Default|GetMTurret) "/Game/AutoMortar/mortar_dome.mortar_dome")
  (Components|StaticMesh|SetStaticMesh (Variables|Default|GetMBarrel) "/Game/AutoMortar/mortar_barrel.mortar_barrel"))